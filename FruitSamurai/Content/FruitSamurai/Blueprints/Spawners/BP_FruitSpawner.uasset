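; BP_FruitSpawner repeatedly launches fruit actors for the FruitSamurai game.
; StartSpawning sets a randomly timed timer for SpawnFruit, which re-arms itself with a new random interval after each spawn.
; Each BP_BaseFruit spawns at GetSpawnTransform, and its Fruit component receives an impulse along the actor root's up vector.
; StopSpawning is an empty stub, so nothing here clears the timer.
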(event `StartSpawning`
  (`KismetSystemLibrary.K2_SetTimer` null "SpawnFruit" (`KismetMathLibrary.RandomFloatInRange` (`self.BaseMinSpawnInterval`) (`self.BaseMaxSpawnInterval`))))

(event `StopSpawning`)

(fn `SpawnFruit`
  (bind _returnvalue (`|SpawnActorFromClass` "/Game/FruitSamurai/Blueprints/Fruits/BP_BaseFruit.BP_BaseFruit_C" (`self.GetSpawnTransform`) "Undefined" "OverrideRootScale" null null))
  (`PrimitiveComponent.AddImpulse` (`/Game/FruitSamurai/Blueprints/Fruits/BP_BaseFruit.Fruit` _returnvalue) (* (`SceneComponent.GetUpVector` (`Actor.RootComponent` _returnvalue)) (`self.SpawnImpulseMagnitude`)) "None" false)
  (`KismetSystemLibrary.K2_SetTimer` null "SpawnFruit" (`KismetMathLibrary.RandomFloatInRange` (`self.BaseMinSpawnInterval`) (`self.BaseMaxSpawnInterval`))))

(fn `UserConstructionScript`)