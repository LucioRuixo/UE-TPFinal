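; Player controller for the fruit-slicing game, handling mouse swipe slicing, score and defeat.
; A swipe begun off fruit traces under the cursor each tick, recording entry and exit points as it crosses a fruit.
; A slice destroys the fruit and updates score, slice balance and threshold through event dispatchers; decreasing the balance to zero triggers defeat.
; Procedural mesh slicing with an impulse exists but is disconnected.
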(event `self.ReceiveBeginPlay`
  (set `self.bShowMouseCursor` true))

(event `self.ReceiveTick`
  (params (DeltaSeconds :type "Float (single-precision)"))
  (bind _hitresult (`self.GetHitResultUnderCursorByChannel` "TraceTypeQuery2"))
  (if (`self.CanSlice`)
    (if (`self.Slicing`)
      (`/Engine/EditorBlueprintResources/StandardMacros.IsValid` (`self.FruitBeingSliced`)
        (:`Is Valid`
          (if (`self.ShouldFruitBeSliced`)
            (`self.SliceFruit` (`self.SliceEnterPoint`) (`self.SliceExitPoint`))))
        (:`Is Not Valid`
          (bind _asbp_base_fruit (cast `/Game/FruitSamurai/Core/Gameplay/Fruits/BP_BaseFruit` (`.HitActor` (`GameplayStatics.BreakHitResult` _hitresult))))
          (set `self.FruitBeingSliced` _asbp_base_fruit)
          (set `self.SliceEnterPoint` (`.Location` (`GameplayStatics.BreakHitResult` _hitresult)))
          (set `self.LastSliceHitPoint` (`.Location` (`GameplayStatics.BreakHitResult` _hitresult)))))
      (else
        (`/Engine/EditorBlueprintResources/StandardMacros.IsValid` null
          (:`Is Valid`
            (set `self.FruitBeingSliced` null)))))))

(event `Key|LeftMouseButton`
  (params (Key :type "Key Structure"))
  (:`Pressed`
    (cast `/Game/FruitSamurai/Core/Gameplay/Fruits/BP_BaseFruit` (`.HitActor` (`GameplayStatics.BreakHitResult` (`self.GetHitResultUnderCursorByChannel` "TraceTypeQuery2")))
      (:`CastFailed`
        (set `self.Slicing` true))))
  (:`Released`
    (set `self.Slicing` false)))

(fn `DecreaseSliceDifference`
  (`|ExecutionSequence`
    (:`then_0`
      (if (> (`self.SliceDifference`) 0)
        (bind _output_get (set `self.SliceDifference` (- (`self.SliceDifference`) 1)))
        (`self.OnSliceDifferenceUpdated` (/ (`KismetMathLibrary.Conv_IntToDouble` _output_get) (`KismetMathLibrary.Conv_IntToDouble` (`self.MaxSliceDifference`))))))
    (:`then_1`
      (if (and (== (`self.SliceDifference`) 0) (`self.CanSlice`))
        (set `self.CanSlice` false)
        (`self.OnDefeat`)
        (`self.OnFinalScoreSet` (`self.Score`))))))

(fn `GetSlicePlaneElements`
  (params (EnterPoint :type "Vector Structure") (ExitPoint :type "Vector Structure"))
  (returns (Position :type "Vector Structure") (Normal :type "Vector Structure"))
  (return (`SceneComponent.K2_GetComponentLocation` (`/Game/FruitSamurai/Core/Gameplay/Fruits/BP_BaseFruit.ProceduralMesh` (`self.FruitBeingSliced`))) (`KismetMathLibrary.Normal` (`KismetMathLibrary.GreaterGreater_VectorRotator` (- ExitPoint EnterPoint) (struct :`Roll` 90.0)))))

(fn `IncreaseSliceDifference`
  (`|ExecutionSequence`
    (:`then_0`
      (if (< (`self.SliceDifference`) (`self.MaxSliceDifference`))
        (bind _output_get (set `self.SliceDifference` (+ (`self.SliceDifference`) 1)))
        (`self.OnSliceDifferenceUpdated` (/ (`KismetMathLibrary.Conv_IntToDouble` _output_get) (`KismetMathLibrary.Conv_IntToDouble` (`self.MaxSliceDifference`))))))
    (:`then_1`
      (bind _output_get_2 (set `self.SlicesMade` (+ (`self.SlicesMade`) 1)))
      (if (>= _output_get_2 (`self.SliceThreshold`))
        (`self.OnSliceThresholdReached`)))))

(fn `ShouldFruitBeSliced`
  (returns (FruitShouldBeCut :type Boolean))
  (bind _hitresult (`self.GetHitResultUnderCursorByChannel` "TraceTypeQuery2"))
  (if (`KismetSystemLibrary.IsValid` (`.HitActor` (`GameplayStatics.BreakHitResult` _hitresult)))
    (bind _asbp_base_fruit (cast `/Game/FruitSamurai/Core/Gameplay/Fruits/BP_BaseFruit` (`.HitActor` (`GameplayStatics.BreakHitResult` _hitresult)))
      (:`then`
        (bind _returnvalue (not (`KismetStringLibrary.EqualEqual_StrStr` (`KismetSystemLibrary.GetDisplayName` _asbp_base_fruit) (`KismetSystemLibrary.GetDisplayName` (`self.FruitBeingSliced`)))))
        (if _returnvalue
          (set `self.SliceExitPoint` (`self.LastSliceHitPoint`))
          (else
            (set `self.LastSliceHitPoint` (`.Location` (`GameplayStatics.BreakHitResult` _hitresult)))))
        (return _returnvalue))
      (:`CastFailed`
        _)))
  (set `self.SliceExitPoint` (`self.LastSliceHitPoint`))
  (return true))

(fn `SliceFruit`
  (params (EnterPoint :type "Vector Structure") (ExitPoint :type "Vector Structure"))
  (`self.K2_DestroyActor` (`self.FruitBeingSliced`))
  (set `self.FruitBeingSliced` null)
  (`self.IncreaseSliceDifference`)
  (bind _output_get (set `self.Score` (+ (`self.Score`) (`self.ScoreIncrement`))))
  (`self.OnFruitCut` _output_get))

(fn `UserConstructionScript`)