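; BP_BaseFruit is the base fruit actor for the Fruit Samurai game, handling despawn and penalties for missed fruit.
; Its construction script copies the static mesh into a procedural mesh component with collision.
; Each tick it checks whether the procedural mesh has fallen to the despawn height, then destroys the actor.
; If the fruit was not sliced, it first calls DecreaseSliceDifference on BP_PlayerController.
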(event `self.ReceiveTick`
  (params (DeltaSeconds :type "Float (single-precision)"))
  (bind (_returnvalue_x _returnvalue_y _returnvalue_z) (`KismetMathLibrary.BreakVector` (`SceneComponent.K2_GetComponentLocation` (`self.ProceduralMesh`))))
  (if (<= _returnvalue_z (`self.ZDespawnThreshold`))
    (if (not (`self.Sliced`))
      (bind _asbp_player_controller (cast `/Game/FruitSamurai/Core/Gameplay/Controllers/BP_PlayerController` (`GameplayStatics.GetPlayerController` 0)))
      (`/Game/FruitSamurai/Core/Gameplay/Controllers/BP_PlayerController.DecreaseSliceDifference` _asbp_player_controller))
    (`self.K2_DestroyActor`)))

(fn `UserConstructionScript`
  (`KismetProceduralMeshLibrary.CopyProceduralMeshFromStaticMeshComponent` (`self.StaticMesh`) 0 (`self.ProceduralMesh`) true))