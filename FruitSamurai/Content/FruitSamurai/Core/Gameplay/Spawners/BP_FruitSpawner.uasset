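; Fruit spawner for Fruit Samurai that launches random fruit classes along their up vector with a randomized impulse.
; Once started, SpawnFruit re-arms its own timer at a random interval until spawning is stopped.
; IncreaseSpawnSpeed scales both interval bounds by a multiplier.
; On BeginPlay it binds handlers to the player controller's slice-threshold and defeat events.
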(event `self.ReceiveBeginPlay`
  (bind _asbp_player_controller (cast `/Game/FruitSamurai/Core/Gameplay/Controllers/BP_PlayerController` (`GameplayStatics.GetPlayerController` 0)))
  (add `/Game/FruitSamurai/Core/Gameplay/Controllers/BP_PlayerController.OnSliceThresholdReached` _asbp_player_controller (`|CreateDelegate` :!event `IncreaseSpawnSpeed`))
  (add `/Game/FruitSamurai/Core/Gameplay/Controllers/BP_PlayerController.OnDefeat` _asbp_player_controller (`|CreateDelegate` :!event `StopSpawning`)))

(event `IncreaseSpawnSpeed`
  (set `self.BaseMinSpawnInterval` (* (`self.BaseMinSpawnInterval`) (`self.SpawnIntervalMultiplier`)))
  (set `self.BaseMaxSpawnInterval` (* (`self.BaseMaxSpawnInterval`) (`self.SpawnIntervalMultiplier`))))

(event `StartSpawning`
  (set `self.Spawning` true)
  (`KismetSystemLibrary.K2_SetTimer` null "SpawnFruit" (`KismetMathLibrary.RandomFloatInRange` (`self.BaseMinSpawnInterval`) (`self.BaseMaxSpawnInterval`))))

(event `StopSpawning`
  (set `self.Spawning` false))

(fn `SpawnFruit`
  (bind _fruitclasses (`self.FruitClasses`))
  (bind _returnvalue (`|SpawnActorFromClass` (`|GetArrayItem` _fruitclasses (`KismetMathLibrary.RandomIntegerInRange` 0 (- (`KismetArrayLibrary.Array_Length` _fruitclasses) 1))) (`self.GetSpawnTransform`) "Undefined" "OverrideRootScale" null null))
  (bind _proceduralmesh (`/Game/FruitSamurai/Core/Gameplay/Fruits/BP_BaseFruit.ProceduralMesh` _returnvalue))
  (`PrimitiveComponent.AddImpulse` _proceduralmesh (* (`SceneComponent.GetUpVector` _proceduralmesh) (`KismetMathLibrary.RandomFloatInRange` (`self.MinSpawnImpulseMagnitude`) (`self.MaxSpawnImpulseMagnitude`))) "None" true)
  (if (`self.Spawning`)
    (`KismetSystemLibrary.K2_SetTimer` null "SpawnFruit" (`KismetMathLibrary.RandomFloatInRange` (`self.BaseMinSpawnInterval`) (`self.BaseMaxSpawnInterval`)))))

(fn `UserConstructionScript`)