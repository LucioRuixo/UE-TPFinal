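; GM_Gameplay is the Fruit Samurai game mode that sets up a play session and controls when fruit spawns.
; On BeginPlay it spawns a player camera and a fruit spawner at the origin if missing, then calls StartGame.
; The camera becomes the first player's view target.
; The OnStartGame and OnEndGame events start and stop the spawner.
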(event `self.ReceiveBeginPlay`
  (`self.SetUpCamera`)
  (`self.SetUpSpawners`)
  (`self.StartGame`))

(event `self.OnStartGame`
  (`/Game/FruitSamurai/Core/Gameplay/Spawners/BP_FruitSpawner.StartSpawning` (`self.FruitSpawner`)))

(event `self.OnEndGame`
  (`/Game/FruitSamurai/Core/Gameplay/Spawners/BP_FruitSpawner.StopSpawning` (`self.FruitSpawner`)))

(fn `SetUpCamera`
  (`/Engine/EditorBlueprintResources/StandardMacros.IsValid` (`self.Camera`)
    (:`Is Not Valid`
      (bind _returnvalue (`|SpawnActorFromClass` "/Game/FruitSamurai/Core/Gameplay/Cameras/BP_PlayerCamera.BP_PlayerCamera_C" (`KismetMathLibrary.MakeTransform` (0.0 0.0 0.0)) "Undefined" "OverrideRootScale" null null))
      (bind _output_get (set `self.Camera` _returnvalue))
      (`PlayerController.SetViewTargetWithBlend` (`GameplayStatics.GetPlayerController` 0) _output_get 0.0 "VTBlend_Linear" 0.0 false))))

(fn `SetUpSpawners`
  (`/Engine/EditorBlueprintResources/StandardMacros.IsValid` (`self.FruitSpawner`)
    (:`Is Not Valid`
      (bind _returnvalue (`|SpawnActorFromClass` "/Game/FruitSamurai/Core/Gameplay/Spawners/BP_FruitSpawner.BP_FruitSpawner_C" (`KismetMathLibrary.MakeTransform` (0.0 0.0 0.0)) "Undefined" "OverrideRootScale" null null))
      (set `self.FruitSpawner` _returnvalue))))

(fn `UserConstructionScript`)